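; MyPortal is a portal obstacle that destroys the player's rocket pawn on contact.
; Its inner, outer and triangle components (Unutar, Vani, Trokut) each call DestroyPawn when a Rocket_gamePawn begins overlapping them.
; Every Tick turns the inner component toward TunelLocation at a constant rate, then adds a fixed per-frame roll, writing the world rotation back as relative rotation.
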(event `self.PortalUnutar.OnComponentBeginOverlap`
  (params (OverlappedComponent :type "PrimitiveComponent Object Reference") (OtherActor :type "Actor Object Reference") (OtherComp :type "PrimitiveComponent Object Reference") (OtherBodyIndex :type Integer) (bFromSweep :type Boolean) (SweepResult :type "HitResult Structure (by ref)"))
  (bind _asrocket_game_pawn (cast `Rocket_gamePawn` OtherActor))
  (`Rocket_gamePawn.Destroy_Pawn` _asrocket_game_pawn))

(event `self.PortalVani.OnComponentBeginOverlap`
  (params (OverlappedComponent :type "PrimitiveComponent Object Reference") (OtherActor :type "Actor Object Reference") (OtherComp :type "PrimitiveComponent Object Reference") (OtherBodyIndex :type Integer) (bFromSweep :type Boolean) (SweepResult :type "HitResult Structure (by ref)"))
  (bind _asrocket_game_pawn (cast `Rocket_gamePawn` OtherActor))
  (`Rocket_gamePawn.Destroy_Pawn` _asrocket_game_pawn))

(event `self.PortalTrokut.OnComponentBeginOverlap`
  (params (OverlappedComponent :type "PrimitiveComponent Object Reference") (OtherActor :type "Actor Object Reference") (OtherComp :type "PrimitiveComponent Object Reference") (OtherBodyIndex :type Integer) (bFromSweep :type Boolean) (SweepResult :type "HitResult Structure (by ref)"))
  (bind _asrocket_game_pawn (cast `Rocket_gamePawn` OtherActor))
  (`Rocket_gamePawn.Destroy_Pawn` _asrocket_game_pawn))

(event `self.ReceiveTick`
  (params (DeltaSeconds :type "Float (single-precision)"))
  (bind _portalunutar (`self.PortalUnutar`))
  (bind _portalunutar_2 (`self.PortalUnutar`))
  (bind (_returnvalue_roll _returnvalue_pitch _returnvalue_yaw) (`KismetMathLibrary.BreakRotator` (`SceneComponent.K2_GetComponentRotation` _portalunutar)))
  (`SceneComponent.K2_SetWorldRotation` (`self.PortalUnutar`) (`KismetMathLibrary.RInterpTo_Constant` (`SceneComponent.K2_GetComponentRotation` _portalunutar_2) (`KismetMathLibrary.FindLookAtRotation` (`SceneComponent.K2_GetComponentLocation` _portalunutar_2) (`self.TunelLocation`)) (`GameplayStatics.GetWorldDeltaSeconds`) 150.0) false false)
  (`SceneComponent.K2_SetRelativeRotation` _portalunutar (`KismetMathLibrary.MakeRotator` (+ _returnvalue_roll 2.0) _returnvalue_pitch _returnvalue_yaw) false false))

(fn `UserConstructionScript`)