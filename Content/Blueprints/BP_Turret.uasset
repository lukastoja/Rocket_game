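; Turret actor that picks a Target every tick through FindBestTarget, with no aiming or firing logic in these graphs.
; The only candidate is player pawn 0, since a SphereOverlapActors search for pawns within SensingRange is left disconnected.
; A candidate needs line of sight from StaticMeshTop and must be closer than the current best.
; The distance test is bypassed while no best target exists, so SensingRange does not limit that pick.
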(event `self.ReceiveTick`
  (params (DeltaSeconds :type "Float (single-precision)"))
  (`self.FindBestTarget`))

(fn `FindBestTarget`
  (locals (`BestDistance (local)` :type "Float (double-precision)") (`CurrentDistance (local)` :type "Float (double-precision)") (`BestTarget (local)` :type "Actor Object Reference") (`CurrentTarget (local)` :type "Actor Object Reference"))
  (set `local.BestDistance (local)` (+ (`self.SensingRange`) 1.0))
  (for _array_element (`|MakeArray` (`GameplayStatics.GetPlayerPawn` 0) :!type "Actor Object Reference")
    (bind _output_get (set `local.CurrentTarget (local)` _array_element))
    (bind _output_get_2 (set `local.CurrentDistance (local)` (`self.GetDistanceTo` _output_get self)))
    (if (or (< _output_get_2 (`local.BestDistance (local)`)) (not (`KismetSystemLibrary.IsValid` (`local.BestTarget (local)`))))
      (bind _result (`/Game/MyFunctionLibrary.HasLineOfSight` (`SceneComponent.K2_GetComponentLocation` (`self.StaticMeshTop`)) (`self.K2_GetActorLocation` (`local.CurrentTarget (local)`)) (`|MakeArray` self (`local.CurrentTarget (local)`) :!type "Actor Object Reference")))
      (if _result
        (set `local.BestTarget (local)` (`local.CurrentTarget (local)`))
        (set `local.BestDistance (local)` (`local.CurrentDistance (local)`)))))
  (set `self.Target` (`local.BestTarget (local)`)))

(fn `UserConstructionScript`)